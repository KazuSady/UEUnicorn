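; BP_DynamicBuilding is a building actor whose Cube mesh material follows the active mapping.
; On BeginPlay it subscribes to MappingManager's mapping-changed event and immediately applies the manager's current state.
; When a mapping name found in its Mappings collection becomes active, it sets the supplied building material on the cube's first slot; other mappings leave the material unchanged.
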(event `HandleMappingChanged`
  (params (NewMappingName :type Name) (NewMaterial :type "Material Object Reference") (NewBuldingMat :type "Material Object Reference"))
  (if (`KismetArrayLibrary.Array_Contains` (`self.Mappings`) NewMappingName)
    (`PrimitiveComponent.SetMaterial` (`self.Cube`) 0 NewBuldingMat)))

(event `self.ReceiveBeginPlay`
  (bind _mappingmanager (`self.MappingManager`))
  (`/Engine/EditorBlueprintResources/StandardMacros.IsValid` _mappingmanager
    (:`Is Valid`
      (add `/Game/Blueprints/BP_MappingManager.OnMappingChanged` _mappingmanager (delegate `HandleMappingChanged`))
      (`self.HandleMappingChanged` (`/Game/Blueprints/BP_MappingManager.CurrentMapping` _mappingmanager) (`/Game/Blueprints/BP_MappingManager.CurrentMaterial` _mappingmanager) (`/Game/Blueprints/BP_MappingManager.CurrentBuildingMaterial` _mappingmanager)))))

(fn `UserConstructionScript`)