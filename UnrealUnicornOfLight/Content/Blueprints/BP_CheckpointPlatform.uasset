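; Checkpoint platform that switches between a solid mesh and a non-active state based on whether the current mapping is in its ActiveMappings list.
; HandleMappingChanged applies the new material and calls UpdatePlatformState, which toggles mesh visibility and collision and shows the Box only while inactive.
; The MappingManager binding and initial sync are disconnected from BeginPlay, marked temporarily disabled, so the platform does not currently react to mapping changes by itself.
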(event `HandleMappingChanged`
  (params (NewMappingName :type Name) (NewMaterial :type "Material Object Reference") (NewBuldingMat :type "Material Object Reference"))
  (`self.UpdatePlatformState` (`KismetArrayLibrary.Array_Contains` (`self.ActiveMappings`) NewMappingName))
  (`PrimitiveComponent.SetMaterial` (`self.PlatformMesh`) 0 NewMaterial))

(event `self.ReceiveBeginPlay`)

(fn `UpdatePlatformState`
  (params (bIsActive :type Boolean))
  (bind _platformmesh (`self.PlatformMesh`))
  (`SceneComponent.SetHiddenInGame` (`self.Box`) bIsActive false)
  (`SceneComponent.SetHiddenInGame` _platformmesh (not bIsActive) false)
  (`PrimitiveComponent.SetCollisionEnabled` _platformmesh (select `bool` bIsActive :`false` "NoCollision" :`true` "QueryAndPhysics" :!type "ECollisionEnabled Enum")))

(fn `UserConstructionScript`)