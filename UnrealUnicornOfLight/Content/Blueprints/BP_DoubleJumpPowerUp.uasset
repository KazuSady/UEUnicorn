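; BP_DoubleJumpPowerUp is a pickup actor that enables double jump on the UnicornCharacter that overlaps it.
; On overlap it calls ToggleDoubleJump, plays a 2D sound, prints a green confirmation message and destroys itself.
; Every tick it bobs vertically by adding a sine of game time to its Z location, an offset per frame that depends on frame rate.
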(event `self.ReceiveActorBeginOverlap`
  (params (OtherActor :type "Actor Object Reference"))
  (bind _asunicorn_character (cast `UnicornCharacter` OtherActor))
  (`UnicornCharacter.ToggleDoubleJump` _asunicorn_character true)
  (`GameplayStatics.PlaySound2D` "/Engine/VREditor/Sounds/UI/Floating_UI_Open.Floating_UI_Open" 1.0 1.0 0.0 null null)
  (`KismetSystemLibrary.PrintString` "Double Jump Enabled!" true true (struct :`G` 1.0 :`A` 1.0) 2.0 "Double Jump Enabled!")
  (`self.K2_DestroyActor`))

(event `self.ReceiveTick`
  (params (DeltaSeconds :type "Float (single-precision)"))
  (`self.K2_SetActorLocation` (`KismetMathLibrary.MakeVector` (.x (`self.K2_GetActorLocation`)) (.y (`self.K2_GetActorLocation`)) (+ (.z (`self.K2_GetActorLocation`)) (`KismetMathLibrary.Sin` (* (`KismetSystemLibrary.GetGameTimeInSeconds`) 10.0))))))

(fn `UserConstructionScript`)