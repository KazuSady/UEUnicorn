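; BP_MappingManager cycles the active mapping, with its matching material and building material, on a timer or an E press.
; Each switch broadcasts the new name and materials through the OnMappingChanged dispatcher, then restarts the timer.
; Its own handler calls ToggleEnemy on walking enemies cached at BeginPlay, based on whether their MappingTag matches.
; That handler binds after the initial switch, so it misses the first broadcast.
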(event `SwitchToNextMapping`
  (bind _mappingcycle (`self.MappingCycle`))
  (bind _output_get (set `self.CurrentMappingIndex` (mod (+ (`self.CurrentMappingIndex`) 1) (`KismetArrayLibrary.Array_Length` _mappingcycle))))
  (bind _output_get_2 (set `self.CurrentMapping` (`|GetArrayItem` _mappingcycle _output_get)))
  (bind _output_get_3 (set `self.CurrentMaterial` (`|GetArrayItem` (`self.Materials`) _output_get)))
  (bind _output_get_4 (set `self.CurrentBuildingMaterial` (`|GetArrayItem` (`self.BuildingMaterials`) _output_get)))
  (`self.OnMappingChanged` _output_get_2 _output_get_3 _output_get_4)
  (`KismetSystemLibrary.PrintString` (`KismetStringLibrary.BuildString_Name` "SwitchToNextMapping" ": " _output_get_2))
  (`KismetSystemLibrary.K2_ClearAndInvalidateTimerHandle` (`self.MappingTimerHandle`))
  (bind _returnvalue (`KismetSystemLibrary.K2_SetTimerDelegate` (delegate `OnTimerFired`) (`self.TimePerMapping`)))
  (set `self.MappingTimerHandle` _returnvalue))

(event `OnTimerFired`
  (`self.SwitchToNextMapping`))

(event `self.ReceiveBeginPlay`
  (`self.EnableInput` self (`GameplayStatics.GetPlayerController` 0))
  (bind _outactors (`GameplayStatics.GetAllActorsOfClass` "/Game/Blueprints/BP_WalkingEnemy.BP_WalkingEnemy_C"))
  (set `self.EnemyRefs` _outactors)
  (if (> (`KismetArrayLibrary.Array_Length` (`self.MappingCycle`)) 0)
    (`self.SwitchToNextMapping`)
    (add `self.OnMappingChanged` (delegate `OnMappingChanged_Event`))
    (else
      (`KismetSystemLibrary.PrintString` "Warning: \"MappingCycle is empty on BP_MappingManager! System will not run.\""))))

(event `Key|E`
  (params (Key :type "Key Structure"))
  (:`Pressed`
    (`self.SwitchToNextMapping`)))

(event `OnMappingChanged_Event`
  (params (NewMappingName :type Name) (NewMaterial :type "Material Object Reference") (NewBuldingMat :type "Material Object Reference"))
  (for _array_element (`self.EnemyRefs`)
    (bind _mappingtag (`/Game/Blueprints/BP_WalkingEnemy.MappingTag` _array_element))
    (`KismetSystemLibrary.PrintString` (`KismetStringLibrary.Conv_NameToString` _mappingtag))
    (`/Game/Blueprints/BP_WalkingEnemy.Toggle Enemy` _array_element (== _mappingtag NewMappingName))))

(fn `UserConstructionScript`)