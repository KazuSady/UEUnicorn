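; Walking enemy that patrols back and forth along the world Y axis and damages the unicorn character on contact.
; Each tick it moves without sweep and traces downward ahead of itself, reversing direction and rotating half a turn when no ground is found.
; Its Box overlap applies damage to BP_NewUnicorn.
; ToggleEnemy switches visibility, collision and ticking together to enable or disable it.
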(event `self.ReceiveBeginPlay`
  (set `self.MovementDirection` 1.0))

(event `self.ReceiveTick`
  (params (DeltaSeconds :type "Float (single-precision)"))
  (bind _x (.x (`self.K2_GetActorLocation`)))
  (bind _z (.z (`self.K2_GetActorLocation`)))
  (bind _returnvalue (+ (* (`self.MovementDirection`) (`self.EdgeDetectionRange`)) (.y (`self.K2_GetActorLocation`))))
  (`self.K2_AddActorWorldOffset` (`KismetMathLibrary.MakeVector` 0.0 (* DeltaSeconds (* (`self.MovementDirection`) (`self.Speed`)))))
  (bind (_outhit _returnvalue_2) (`KismetSystemLibrary.LineTraceSingle` (`KismetMathLibrary.MakeVector` _x _returnvalue _z) (`KismetMathLibrary.MakeVector` _x _returnvalue (- _z 100.0)) "TraceTypeQuery1"))
  (if (not _returnvalue_2)
    (set `self.MovementDirection` (* (`self.MovementDirection`) -1.0))
    (`self.K2_AddActorLocalRotation` (struct :`Yaw` 180.0))))

(event `self.Box.OnComponentBeginOverlap`
  (params (OverlappedComponent :type "PrimitiveComponent Object Reference") (OtherActor :type "Actor Object Reference") (OtherComp :type "PrimitiveComponent Object Reference") (OtherBodyIndex :type Integer) (bFromSweep :type Boolean) (SweepResult :type "HitResult Structure (by ref)"))
  (bind _asbp_new_unicorn (cast `/Game/Blueprints/BP_NewUnicorn` OtherActor))
  (`UnicornCharacter.TakeDamage` _asbp_new_unicorn 1))

(fn `Toggle Enemy`
  (params (`Is Enabled` :type Boolean))
  (bind _bisenabled (`self.bIsEnabled`))
  (set `self.bIsEnabled` `Is Enabled`)
  (`self.SetActorHiddenInGame` (not _bisenabled))
  (`self.SetActorEnableCollision` _bisenabled)
  (`self.SetActorTickEnabled` _bisenabled))

(fn `UserConstructionScript`)