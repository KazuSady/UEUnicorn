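; UnicornController is the player controller that handles movement and jump input for the UnicornBP character.
; On BeginPlay it sets game-only input, caches the controlled pawn as UnicornBP and adds the Enhanced Input mapping context.
; IA_Move adds movement along the character's forward vector, scaled by the action value.
; IA_Jump starts a jump when pressed and stops it on completion or cancellation.
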(event `self.ReceiveBeginPlay`
  (`WidgetBlueprintLibrary.SetInputMode_GameOnly` self)
  (bind _asunicorn_bp (cast `/Game/Blueprints/UnicornBP` (`self.K2_GetPawn`)))
  (set `self.UnicornCharacter` _asunicorn_bp)
  (`EnhancedInputSubsystemInterface.AddMappingContext` (subsystem `EnhancedInputLocalPlayerSubsystem`) "/Game/Blueprints/Input/UnicornMappingContext.UnicornMappingContext" 0 (struct)))

(event `EnhancedInput|/Game/Blueprints/Input/IA_Move`
  (params (ActionValue :type "Float (double-precision)") (ElapsedSeconds :type "Float (double-precision)") (TriggeredSeconds :type "Float (double-precision)") (InputAction :type "InputAction Object Reference" :default "/Game/Blueprints/Input/IA_Move.IA_Move"))
  (bind _unicorncharacter (`self.UnicornCharacter`))
  (:`Triggered`
    (`Pawn.AddMovementInput` _unicorncharacter (`self.GetActorForwardVector` _unicorncharacter) ActionValue false)))

(event `EnhancedInput|/Voxel/Examples/CubicDestruction/Actions/IA_Jump`
  (params (ActionValue :type Boolean) (ElapsedSeconds :type "Float (double-precision)") (TriggeredSeconds :type "Float (double-precision)") (InputAction :type "InputAction Object Reference" :default "/Voxel/Examples/CubicDestruction/Actions/IA_Jump.IA_Jump"))
  (bind _unicorncharacter (`self.UnicornCharacter`))
  (:`Started`
    (`Character.Jump` _unicorncharacter))
  (:`Canceled`
    (`Character.StopJumping` _unicorncharacter :!label _label))
  (:`Completed`
    (goto _label)))

(fn `UserConstructionScript`)