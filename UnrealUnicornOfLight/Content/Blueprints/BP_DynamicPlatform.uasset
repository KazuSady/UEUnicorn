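; BP_DynamicPlatform is a platform that appears or disappears depending on the current mapping.
; It binds to its MappingManager's mapping-changed event on BeginPlay and immediately applies the manager's current state.
; Each change toggles mesh visibility and collision by checking the name against ActiveMappings, then applies the new material, ignoring the building material.
; Without a valid manager, it prints a warning and stays hidden without collision.
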(event `HandleMappingChanged`
  (params (NewMappingName :type Name) (NewMaterial :type "Material Object Reference") (NewBuldingMat :type "Material Object Reference"))
  (`self.UpdatePlatformState` (`KismetArrayLibrary.Array_Contains` (`self.ActiveMappings`) NewMappingName))
  (`PrimitiveComponent.SetMaterial` (`self.PlatformMesh`) 0 NewMaterial))

(event `self.ReceiveBeginPlay`
  (bind _mappingmanager (`self.MappingManager`))
  (`/Engine/EditorBlueprintResources/StandardMacros.IsValid` _mappingmanager
    (:`Is Valid`
      (add `/Game/Blueprints/BP_MappingManager.OnMappingChanged` _mappingmanager (delegate `HandleMappingChanged`))
      (`self.HandleMappingChanged` (`/Game/Blueprints/BP_MappingManager.CurrentMapping` _mappingmanager) (`/Game/Blueprints/BP_MappingManager.CurrentMaterial` _mappingmanager) (`/Game/Blueprints/BP_MappingManager.CurrentBuildingMaterial` _mappingmanager)))
    (:`Is Not Valid`
      (`KismetSystemLibrary.PrintString` "Warning: \"No Mapping Manager assigned!\"")
      (`self.UpdatePlatformState` false))))

(fn `UpdatePlatformState`
  (params (bIsActive :type Boolean))
  (bind _platformmesh (`self.PlatformMesh`))
  (`SceneComponent.SetHiddenInGame` _platformmesh (not bIsActive) false)
  (`PrimitiveComponent.SetCollisionEnabled` _platformmesh (select `bool` bIsActive :`false` "NoCollision" :`true` "QueryAndPhysics" :!type "ECollisionEnabled Enum")))

(fn `UserConstructionScript`)